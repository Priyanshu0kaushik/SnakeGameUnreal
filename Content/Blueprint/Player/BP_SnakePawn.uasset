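; BP_SnakePawn is the player-controlled snake pawn, translating Enhanced Input actions into movement requests.
; On BeginPlay it adds the IMC_Player1 mapping context to its player controller's input subsystem.
; The four move actions pass their direction to AddDirectionToQueue, so turns are queued, while the jump action prints a debug "Hello" and calls Jump.
; Neither the queue nor the jump logic is defined in this Blueprint.
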(event Input|EnhancedActionEvents|EnhancedInputActionIA_MoveUP
  (params (ActionValue :type Boolean) (ElapsedSeconds :type Float%20%28double-precision%29) (TriggeredSeconds :type Float%20%28double-precision%29) (InputAction :type Input%20Action%20Object%20Reference :default "/Game/Input/Actions/IA_MoveUP.IA_MoveUP"))
  ;[0.15 0.15 0.15 0.5] Input Actions
  (Class|SnakePawn|AddDirectiontoQueue "UP"))

(event Input|EnhancedActionEvents|EnhancedInputActionIA_MoveDOWN
  (params (ActionValue :type Boolean) (ElapsedSeconds :type Float%20%28double-precision%29) (TriggeredSeconds :type Float%20%28double-precision%29) (InputAction :type Input%20Action%20Object%20Reference :default "/Game/Input/Actions/IA_MoveDOWN.IA_MoveDOWN"))
  ;[0.15 0.15 0.15 0.5] Input Actions
  (Class|SnakePawn|AddDirectiontoQueue "DOWN"))

(event Input|EnhancedActionEvents|EnhancedInputActionIA_MoveRIGHT
  (params (ActionValue :type Boolean) (ElapsedSeconds :type Float%20%28double-precision%29) (TriggeredSeconds :type Float%20%28double-precision%29) (InputAction :type Input%20Action%20Object%20Reference :default "/Game/Input/Actions/IA_MoveRIGHT.IA_MoveRIGHT"))
  ;[0.15 0.15 0.15 0.5] Input Actions
  (Class|SnakePawn|AddDirectiontoQueue "RIGHT"))

(event Input|EnhancedActionEvents|EnhancedInputActionIA_MoveLEFT
  (params (ActionValue :type Boolean) (ElapsedSeconds :type Float%20%28double-precision%29) (TriggeredSeconds :type Float%20%28double-precision%29) (InputAction :type Input%20Action%20Object%20Reference :default "/Game/Input/Actions/IA_MoveLEFT.IA_MoveLEFT"))
  ;[0.15 0.15 0.15 0.5] Input Actions
  (Class|SnakePawn|AddDirectiontoQueue "LEFT"))

(event Input|EnhancedActionEvents|EnhancedInputActionIA_Jump
  (params (ActionValue :type Boolean) (ElapsedSeconds :type Float%20%28double-precision%29) (TriggeredSeconds :type Float%20%28double-precision%29) (InputAction :type Input%20Action%20Object%20Reference :default "/Game/Input/Actions/IA_Jump.IA_Jump"))
  ;[0.15 0.15 0.15 0.5] Input Actions
  (Development|PrintString "Hello")
  (Class|SnakePawn|Jump))

(event EventBeginPlay
  (bind _asplayer_controller (Utilities|Casting|CastToPlayerController (Pawn|GetController)))
  (Input|AddMappingContext (PlayerController|LocalPlayerSubsystems|GetEnhancedInputLocalPlayerSubsystem _asplayer_controller) "/Game/Input/IMC_Player1.IMC_Player1" 0 "(bIgnoreAllPressedKeysUntilRelease=True,bForceImmediately=False,bNotifyUserSettings=False)"))

(event Collision|EventActorBeginOverlap
  (params (OtherActor :type Actor%20Object%20Reference)))

(event EventTick
  (params (DeltaSeconds :type Float%20%28single-precision%29)))

(fn ConstructionScript)